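; Bp_IA is an AI pawn that wanders between random reachable points and chases the player when it sees a pawn.
; Each successful wander move picks another point within a 1000-unit radius of its current location.
; PawnSensing sightings start a move to player 0, and a retriggerable one-second delay resumes wandering once sightings stop.
; The AIPerception update handler loops without acting.
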(event OnSeePawn(PawnSensing)
  (params (Pawn :type Pawn%20Object%20Reference))
  (Utilities|FlowControl|Sequence
    (:then_0
      (AI|AIMoveTo self "0, 0, 0" (Game|Player|GetPlayerPawn 0) 5.0 false))
    (:then_1
      (Utilities|FlowControl|RetriggerableDelay 1.0)
      (CallFunction|GotoRamdomPoint))))

(event OnPerceptionUpdated(AIPerception)
  (params (UpdatedActors :type Array%20of%20Actor%20Object%20References))
  (Class|AIPerceptionComponent|GetActorsPerception (Variables|Default|GetAIPerception))
  (for _array_element 0
    _))

(event Custom|GoToRamdomPoint
  (AI|AIMoveTo self (.RandomLocation (AI|Navigation|GetRandomReachablePointinRadius (Transformation|GetActorLocation) 1e+03 0 0)) 0 5.0 false
    (:OnSuccess
      (CallFunction|GotoRamdomPoint))))

(event EventBeginPlay
  (CallFunction|GotoRamdomPoint))

(fn ConstructionScript)